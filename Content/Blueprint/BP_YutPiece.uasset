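; Yut board game piece actor that glides to a target road's PieceLocation when MoveToRoad is called.
; MoveToRoad returns false if a move is already running; otherwise it stores the target and starts a looping timer at about 60 Hz instead of using Tick.
; Each timer cycle eases the actor toward the target with VInterpTo, then snaps within a small tolerance, clears the timer and resets the moving flag.
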(event EventBeginPlay)

(event Collision|EventActorBeginOverlap
  (params (OtherActor :type Actor%20Object%20Reference)))

(event EventTick
  (params (DeltaSeconds :type Float%20%28single-precision%29)))

(fn ConstructionScript)

(fn MovetoRoad
  (params (ToRoad :type BP%20Yut%20Board%20Road%20Object%20Reference))
  (bind _bsuccessmoving (CallFunction|MovetoRoadStart (Transformation|GetWorldLocation (Variables|/Game/Blueprint/BP_YutBoardRoad.BP_YutBoardRoad_C|GetPieceLocation ToRoad))))
  (return _bsuccessmoving))

(fn MovetoRoadStart
  (params (NewLocation :type Vector))
  (Variables|Default|GetbIsMoving
    (:then
      (return false))
    (:else
      (Variables|Default|SetbIsMoving true)
      (Variables|Default|SetTargetLocation NewLocation)
      (bind _returnvalue (Utilities|Time|SetTimerbyFunctionName 0 "MoveToRoad_Cycle" 0.0166 true))
      (Variables|Default|SetTH_Moving _returnvalue)
      (return true))))

(fn MovetoRoadCycle
  (Transformation|SetActorLocation (Math|Interpolation|VInterpTo (Transformation|GetActorLocation) (Variables|Default|GetTargetLocation) (Utilities|Time|GetWorldDeltaSeconds) 5.0) false true)
  (if (Utilities|Operators|EqualEqual (Transformation|GetActorLocation) (Variables|Default|GetTargetLocation) 2.0)
    (Transformation|SetActorLocation (Variables|Default|GetTargetLocation) false true)
    (Utilities|Time|ClearandInvalidateTimerbyHandle (Variables|Default|GetTH_Moving))
    (CallFunction|MovetoRoadFinish)))

(fn MovetoRoadFinish
  (Variables|Default|SetbIsMoving false))